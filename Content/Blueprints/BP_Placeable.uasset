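; BP_Placeable is an actor that follows the cursor while it is being placed.
; StartPlacing stores the controller, sets the placing flag and calls EditMaterial, which is an empty stub here; StopPlacing clears the flag.
; While placing, Tick traces under the cursor against the configured object types and snaps the actor to the hit component's world location rather than the exact hit point.
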(event Custom|Start%20Placing
  (params (Controller :type Player%20Controller%20Object%20Reference))
  (Variables|Default|SetController Controller)
  (Variables|Default|SetIsBeingPlaced true)
  (CallFunction|EditMaterial))

(event Custom|Stop%20Placing
  (Variables|Default|SetIsBeingPlaced false))

(event EventBeginPlay)

(event Collision|EventActorBeginOverlap
  (params (OtherActor :type Actor%20Object%20Reference)))

(event EventTick
  (params (DeltaSeconds :type Float%20%28single-precision%29))
  (bind _controller (Variables|Default|GetController))
  (bind _object_types (Variables|Default|GetObject%20Types))
  (bind _hitresult (Class|PlayerController|GetHitResultUnderCursorforObjects _controller _object_types true))
  (bind _hitcomponent (Collision|BreakHitResult _hitresult))
  (if (Variables|Default|GetIsBeingPlaced)
    (if (Utilities|IsValid _hitcomponent)
      (Transformation|SetActorLocation (Transformation|GetWorldLocation _hitcomponent) false false))))

(fn ConstructionScript)

(fn EditMaterial)