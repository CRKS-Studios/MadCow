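; AI controller for a projectile turret that tracks and shoots enemies from a maintained target list.
; TargetsInRange locks onto the first listed target and starts a one-second looping shoot timer, while Tick keeps the turret aimed at that target.
; Each shot requires the current target to still be listed; the timer and lock clear only when the list is empty, with no retargeting before then.
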(event Custom|Event%20TargetsInRange
  (if (not (Variables|Default|GetHasTarget))
    (Variables|Default|SetCurrentTarget (Utilities|Array|Get(acopy) (Variables|Default|GetTargets)))
    (Variables|Default|SetHasTarget true)
    (bind _returnvalue (Utilities|Time|SetTimerbyFunctionName 0 "ShootAtTarget" 1.0 true))
    (Variables|Default|SetShootingTimer _returnvalue)))

(event EventTick
  (params (DeltaSeconds :type Float%20%28single-precision%29))
  ;[1 1 1] Point at nearest enemy
  (if (Variables|Default|GetHasTarget)
    (bind _asbp_abstract_turret (Utilities|Casting|CastToBP_AbstractTurret (Pawn|GetControlledPawn)))
    (Default|LookatLocation _asbp_abstract_turret (Transformation|GetActorLocation (Variables|Default|GetCurrentTarget)))))

(fn ConstructionScript)

(fn AddPotentialTarget
  (params (NewTarget :type Actor%20Object%20Reference))
  (bind _asbp_enemy (Utilities|Casting|CastToBP_Enemy NewTarget))
  (Utilities|Array|Add (Variables|Default|GetTargets) _asbp_enemy))

(fn RemoveTarget
  (params (Target :type BP%20Enemy%20Object%20Reference))
  (Utilities|Array|RemoveItem (Variables|Default|GetTargets) Target))

(fn ShootatTarget
  (if (> (Utilities|Array|Length (Variables|Default|GetTargets)) 0)
    (if (Utilities|Array|ContainsItem (Variables|Default|GetTargets) (Variables|Default|GetCurrentTarget))
      (bind _asbp_projectile_turret (Utilities|Casting|CastToBP_ProjectileTurret (Pawn|GetControlledPawn)))
      (Default|Shoot _asbp_projectile_turret))
    (else
      (Utilities|Time|ClearandInvalidateTimerbyHandle (Variables|Default|GetShootingTimer))
      (Variables|Default|SetHasTarget false))))