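; BP_EnemySpawner is an actor that spawns waves of enemies on a timer, starting after a start delay plus one wave period.
; SpawnWave rolls a random count for each class in the EnemyComposition map of ranges, spawning them at offsets along SpawnOffset from the spawner.
; Each wave re-arms the timer using GetNewPeriod, intended to vary the period randomly within clamped limits.
; StopSpawning clears the timer and disables further waves.
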(event EventBeginPlay
  (bind _returnvalue (Utilities|Time|SetTimerbyFunctionName 0 "SpawnWave" (+ (Variables|SpawnerSettings|GetStartDelay) (Variables|SpawnerSettings|GetWavePeriod)) true))
  (Variables|Default|SetSpawnTimer _returnvalue))

(event Collision|EventActorBeginOverlap
  (params (OtherActor :type Actor%20Object%20Reference)))

(event EventTick
  (params (DeltaSeconds :type Float%20%28single-precision%29)))

(fn ConstructionScript)

(fn SpawnWave
  (if (Variables|Default|GetShouldSpawn)
    (Utilities|FlowControl|Sequence
      (:then_0
        ;[1 1 1] Spawn wave
        (bind _keys (Utilities|Map|Keys (Variables|SpawnerWaveComposition|GetEnemyComposition)))
        (for (_array_element _array_index) _keys
          (bind _output_get (LocalVariables|SetRandomInt (Math|Random|RandomIntegerinRange (.value (.lowerbound (.Value (Utilities|Map|Find (Variables|SpawnerWaveComposition|GetEnemyComposition) _array_element)))) (.value (.upperbound (.Value (Utilities|Map|Find (Variables|SpawnerWaveComposition|GetEnemyComposition) _array_element)))))))
          (for _index (range 1 _output_get)
            (Game|SpawnActorfromClass _array_element (|CalculateTransform _index _array_index (LocalVariables|GetRandomInt)) "AlwaysSpawn" 0 0))))
      (:then_1
        ;[1 1 1] Calculate new wave period and apply it
        (Utilities|Time|ClearandInvalidateTimerbyHandle (Variables|Default|GetSpawnTimer))
        (bind _returnvalue (Utilities|Time|SetTimerbyFunctionName 0 "SpawnWave" (|GetNewPeriod)))
        (Variables|Default|SetSpawnTimer _returnvalue)))
    (else
      (Utilities|Time|ClearandInvalidateTimerbyHandle (Variables|Default|GetSpawnTimer)))))

(fn StopSpawning
  (Utilities|Time|ClearandInvalidateTimerbyHandle (Variables|Default|GetSpawnTimer))
  (Variables|Default|SetShouldSpawn false))