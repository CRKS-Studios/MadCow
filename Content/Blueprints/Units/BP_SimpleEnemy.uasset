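; BP_SimpleEnemy is a basic enemy unit that varies its look on spawn and collapses physically on death.
; BeginPlay calls the parent, applies InitialScale to the actor and gives Body a random mesh from the first three entries of Meshes.
; PerformDeath extends the parent's death logic by enabling physics on Body and setting a short lifespan so the actor removes itself.
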(event EventBeginPlay
  (|CallParentFunction)
  (Transformation|SetActorScale3D (Variables|Default|GetInitialScale))
  (Components|StaticMesh|SetStaticMesh (Variables|Default|GetBody) (Utilities|Array|Get(acopy) (Variables|Default|GetMeshes) (Math|Random|RandomInteger 3))))

(event Collision|EventActorBeginOverlap
  (params (OtherActor :type Actor%20Object%20Reference))
  (|CallParentFunction OtherActor) ; This node is disabled and will not be called.\nDrag off pins to build functionality.
)

(event EventTick
  (params (DeltaSeconds :type Float%20%28single-precision%29))
  (|CallParentFunction DeltaSeconds) ; This node is disabled and will not be called.\nDrag off pins to build functionality.
)

(fn ConstructionScript
  (|CallParentFunction))

(fn PerformDeath
  (|CallParentFunction)
  (Physics|SetSimulatePhysics (Variables|Default|GetBody) true)
  (Actor|SetLifeSpan 2.0))