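; Base enemy unit that targets the first BP_Barn found at BeginPlay, logging if none exists, with health, damage and death handling.
; SetHealth Z-scales remaining and lost meshes as a health bar, which turns toward the player's pawn every tick.
; TakeDamage subtracts through SetHealth, then subtracts Amount again from the updated value to test for death.
; PerformDeath blocks further health changes and disables capsule collision.
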(event EventBeginPlay
  (Utilities|FlowControl|Sequence
    (:then_0
      (Variables|Default|SetMaxHealthBarScale (.z (Variables|/Script/Engine.SceneComponent|GetRelativeScale3D (Variables|Default|GetRemainingHealthMesh)))))
    (:then_1
      (CallFunction|SetHealth (Variables|Enemy|GetMaxHealth)))
    (:then_2
      (bind _outactors (Actor|GetAllActorsOfClass "/Game/Blueprints/Placeables/BP_Barn.BP_Barn_C"))
      (if (> (Utilities|Array|Length _outactors) 0)
        (Variables|Enemy|SetTargetBuilding (Utilities|Array|Get(acopy) _outactors))
        (else
          (Utilities|String|LogString "No barn in the world. Enemy does not have target!"))))))

(event EventTick
  (params (DeltaSeconds :type Float%20%28single-precision%29))
  (Transformation|SetWorldRotation (Variables|Default|GetHealthBarRoot) (Math|Rotator|FindLookatRotation (Transformation|GetWorldLocation (Variables|Default|GetHealthBarRoot)) (Transformation|GetActorLocation (Pawn|GetControlledPawn (Game|GetPlayerController 0)))) false false))

(fn ConstructionScript
  (|CallParentFunction))

(fn TakeDamage
  (params (Amount :type Float%20%28double-precision%29))
  (bind _currenthealth (Variables|Enemy|GetCurrentHealth))
  (bind _returnvalue (- _currenthealth Amount))
  (CallFunction|SetHealth _returnvalue)
  (if (<= _returnvalue 0.0)
    (CallFunction|PerformDeath)))

(fn SetHealth
  (params (NewHealth :type Float%20%28double-precision%29))
  (bind _losthealthmesh (Variables|Default|GetLostHealthMesh))
  (bind _remaininghealthmesh (Variables|Default|GetRemainingHealthMesh))
  (bind _relativescale3d (Variables|/Script/Engine.SceneComponent|GetRelativeScale3D _remaininghealthmesh))
  (bind _relativescale3d_2 (Variables|/Script/Engine.SceneComponent|GetRelativeScale3D _losthealthmesh))
  (if (not (Variables|Enemy|GetIsDead))
    (LocalVariables|SetRatio (/ NewHealth (Variables|Enemy|GetMaxHealth)))
    (Variables|Enemy|SetCurrentHealth NewHealth)
    (Utilities|FlowControl|Sequence
      (:then_0
        (Transformation|SetRelativeScale3D (Variables|Default|GetRemainingHealthMesh) (Math|Vector|MakeVector (.x _relativescale3d) (.y _relativescale3d) (* (LocalVariables|GetRatio) (Variables|Default|GetMaxHealthBarScale)))))
      (:then_1
        (Transformation|SetRelativeScale3D (Variables|Default|GetLostHealthMesh) (Math|Vector|MakeVector (.x _relativescale3d_2) (.y _relativescale3d_2) (* (- 1.0 (LocalVariables|GetRatio)) (Variables|Default|GetMaxHealthBarScale))))))))

(fn PerformDeath
  (Variables|Enemy|SetIsDead true)
  (Collision|SetCollisionEnabled (Variables|Default|GetCapsuleComponent) "NoCollision"))