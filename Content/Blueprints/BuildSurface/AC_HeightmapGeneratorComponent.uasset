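; Actor component that converts a texture into an array of height values, as a custom heightmap.
; GetCustomHeightMap resizes the supplied render target to the texture's size, then draws the texture into it through a dynamic material instance.
; It reads the pixels back and appends each one's averaged, normalized RGB to HeightArray without clearing it first, then returns that array.
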(event EventBeginPlay)

(event EventTick
  (params (DeltaSeconds :type Float%20%28single-precision%29)))

(fn GetCustomHeightMap
  (params (renderTargetToWrite :type Texture%20Render%20Target%202D%20Object%20Reference) (renderTargetMaterialToWrite :type Material%20Object%20Reference) (texture :type Texture%202D%20Object%20Reference))
  (Rendering|ResizeRenderTarget2D renderTargetToWrite (Class|Texture2D|BlueprintGetSizeX texture) (Class|Texture2D|BlueprintGetSizeY texture))
  (LocalVariables|SetRender%20Target renderTargetToWrite)
  (bind _returnvalue (Rendering|Material|CreateDynamicMaterialInstance renderTargetMaterialToWrite "None" "None" :!class /Script/Engine.KismetMaterialLibrary))
  (bind _output_get (LocalVariables|SetInstanceMaterial _returnvalue))
  (Rendering|Material|SetTextureParameterValue _output_get "RenderTargetMaterialTexture" texture)
  (Rendering|DrawMaterialtoRenderTarget (Variables|Default|GetRenderTarget) (LocalVariables|GetInstanceMaterial))
  (bind _outsamples (Class|KismetRenderingLibrary|ReadRenderTarget (Variables|Default|GetRenderTarget) false))
  (for _array_element _outsamples
    (Utilities|Array|Add (LocalVariables|GetHeightArray) (/ (+ (/ (Math|Conversions|ToFloat(Byte) (.B (Math|Color|BreakColor _array_element))) 255.0) (/ (Math|Conversions|ToFloat(Byte) (.G (Math|Color|BreakColor _array_element))) 255.0) (/ (Math|Conversions|ToFloat(Byte) (.R (Math|Color|BreakColor _array_element))) 255.0)) 3.0)))
  (Development|PrintString "sve se doda")
  (return (LocalVariables|GetHeightArray)))