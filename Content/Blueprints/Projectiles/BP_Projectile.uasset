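; BP_Projectile is a projectile actor that damages BP_Enemy actors its Body component hits.
; On BeginPlay it applies a configurable scale and offset to Body and starts a timer that destroys it after its Lifetime.
; A HitEnemies list records each damaged enemy, so the projectile damages each one only once and is not destroyed on impact.
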(event OnComponentHit(Body)
  (params (HitComponent :type Primitive%20Component%20Object%20Reference) (OtherActor :type Actor%20Object%20Reference) (OtherComp :type Primitive%20Component%20Object%20Reference) (NormalImpulse :type Vector :default "0, 0, 0") (Hit :type Hit%20Result%20Structure%20%28by%20ref%29))
  (if (not (Utilities|Array|ContainsItem (Variables|Default|GetHitEnemies) OtherActor))
    (bind _asbp_enemy (Utilities|Casting|CastToBP_Enemy OtherActor))
    (Default|TakeDamage _asbp_enemy (Variables|Projectile|GetDamage))
    (Utilities|Array|Add (Variables|Default|GetHitEnemies) OtherActor)))

(event EventBeginPlay
  ;[1 1 1] Destroy after being spawned
  (Utilities|Time|SetTimerbyFunctionName 0 "Disappear" (Variables|Projectile|GetLifetime))
  (Transformation|SetWorldScale3D (Variables|Default|GetBody) (Variables|Transform|GetWorldScale))
  (Transformation|AddRelativeLocation (Variables|Default|GetBody) (Variables|Transform|GetLocationOffset) false false))

(event Collision|EventActorBeginOverlap
  (params (OtherActor :type Actor%20Object%20Reference)))

(event EventTick
  (params (DeltaSeconds :type Float%20%28single-precision%29)))

(fn ConstructionScript)

(fn Disappear
  (Actor|DestroyActor))