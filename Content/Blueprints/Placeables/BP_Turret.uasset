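; BP_Turret is a placeable turret that aims its parts at a given location.
; It overrides LookAtLocation, calls the parent, then splits the aim between two components.
; Roof turns in world yaw toward the target, while Gun takes only the look-at pitch as relative rotation.
; Construction and EditMaterial defer to the parent, and the event graph has no active logic.
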(event EventBeginPlay)

(event Collision|EventActorBeginOverlap
  (params (OtherActor :type Actor%20Object%20Reference)))

(event EventTick
  (params (DeltaSeconds :type Float%20%28single-precision%29)))

(fn ConstructionScript
  (|CallParentFunction))

(fn EditMaterial
  (|CallParentFunction))

(fn LookatLocation
  (params (LookAt :type Vector :default "0, 0, 0"))
  (|CallParentFunction LookAt)
  (Utilities|FlowControl|Sequence
    (:then_0
      (Transformation|SetRelativeRotation (Variables|Default|Getgun) (Math|Rotator|MakeRotator 0.0 (.pitch (Math|Rotator|FindLookatRotation (Transformation|GetWorldLocation (Variables|Default|Getgun)) LookAt)) 0.0) false false))
    (:then_1
      (Transformation|SetWorldRotation (Variables|Default|GetRoof) (Math|Rotator|MakeRotator 0.0 0.0 (.yaw (Math|Rotator|FindLookatRotation (Transformation|GetWorldLocation (Variables|Default|GetRoof)) LookAt))) false false))))