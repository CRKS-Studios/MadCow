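; BP_Wall is a placeable wall that adds connecting pieces between itself and other walls when placement stops.
; StopPlacing runs the parent logic, then, if the wall is no longer being placed, loops over overlapping BP_Wall actors.
; For each neighbor it creates a sphere static mesh component at runtime, positioned at the midpoint between the two walls.
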(event EventStopPlacing
  (|CallParentFunction)
  (if (not (Variables|Default|GetIsBeingPlaced))
    (for _array_element (Collision|GetOverlappingActors "BP_Wall_C" :!class /Script/Engine.Actor)
      (bind _returnvalue (AddComponent|AddStaticMeshComponent false))
      (Components|StaticMesh|SetStaticMesh _returnvalue "/Game/StarterContent/Shapes/Shape_Sphere.Shape_Sphere")
      (Transformation|SetWorldLocation _returnvalue (+ (Transformation|GetWorldLocation (Variables|Transformation|GetRootComponent)) (/ (- (Transformation|GetActorLocation _array_element) (Transformation|GetWorldLocation (Variables|Transformation|GetRootComponent))) "2.000000,2.000000,2.000000")) false false))))

(fn ConstructionScript
  (|CallParentFunction))