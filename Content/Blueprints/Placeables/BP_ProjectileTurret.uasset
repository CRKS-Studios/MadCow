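; Placeable projectile turret that provides a Shoot function for firing a projectile actor.
; Shoot spawns ProjectileClass at the world-space location and rotation of SocketName on SocketComponent, at unit scale, with the turret as owner and instigator.
; The event graph holds only disabled default events and the construction script just calls its parent, so nothing in this Blueprint triggers Shoot itself.
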(event EventBeginPlay
  (|CallParentFunction) ; This node is disabled and will not be called.\nDrag off pins to build functionality.
)

(event Collision|EventActorBeginOverlap
  (params (OtherActor :type Actor%20Object%20Reference))
  (|CallParentFunction OtherActor) ; This node is disabled and will not be called.\nDrag off pins to build functionality.
)

(event EventTick
  (params (DeltaSeconds :type Float%20%28single-precision%29))
  (|CallParentFunction DeltaSeconds) ; This node is disabled and will not be called.\nDrag off pins to build functionality.
)

(fn ConstructionScript
  (|CallParentFunction))

(fn Shoot
  (bind _self self)
  (bind _socketname (Variables|ProjectileTurret|GetSocketName))
  (bind _socketcomponent (Variables|ProjectileTurret|GetSocketComponent))
  (bind _returnvalue (Transformation|GetSocketTransform _socketcomponent _socketname "RTS_World"))
  (Game|SpawnActorfromClass (Variables|ProjectileTurret|GetProjectileClass) (Math|Transform|MakeTransform (.location _returnvalue) (.rotation _returnvalue)) "Undefined" _self _self))