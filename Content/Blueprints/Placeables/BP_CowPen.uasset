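; BP_CowPen is a placeable pen that holds cows up to a maximum and earns the player money.
; A BeginPlay loop periodically adds income proportional to the cow count to BP_TopDownController's money buffer.
; AddCow spawns a scaled-down, randomly rotated BP_Cow until the pen is full.
; Shuffled slot indices give each cow its own angle around the pen mesh, with a randomised radial offset.
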(event EventBeginPlay
  (bind _occupied (Variables|Default|Getoccupied))
  (for _index (range 1 (Variables|Default|GetMax_Cows))
    (Utilities|Array|Add _occupied _index))
  (Utilities|Array|Shuffle _occupied)
  (Utilities|FlowControl|Delay 5.0 :!label _label)
  (bind _asbp_top_down_controller (Utilities|Casting|CastToBP_TopDownController (Game|GetPlayerController 0)))
  (Default|IncreaseMoneyBuffer _asbp_top_down_controller (Class|KismetMathLibrary|ToInt64(Integer) (* (Variables|Default|GetNumber_Cows) 5)))
  (goto _label))

(event Collision|EventActorBeginOverlap
  (params (OtherActor :type Actor%20Object%20Reference)))

(event EventTick
  (params (DeltaSeconds :type Float%20%28single-precision%29)))

(fn ConstructionScript)

(fn AddCow
  (if (< (Variables|Default|GetNumber_Cows) (Variables|Default|GetMax_Cows))
    (Variables|Default|SetNumber_Cows (+ (Variables|Default|GetNumber_Cows) 1))
    (Game|SpawnActorfromClass "/Game/Blueprints/Units/BP_Cow.BP_Cow_C" (Math|Transform|MakeTransform (stale _returnvalue) (Math|Rotator|MakeRotator 0.0 0.0 (Math|Random|RandomFloatinRange 0.0 3.6e+02)) "0.070000,0.070000,0.070000") "AlwaysSpawn" 0 0)
    (else
      (Development|PrintString "this pen is full!"))))