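; Base turret pawn for placeable turrets that reports targets entering and leaving its range to its AI controller.
; The construction script sizes the range sphere from TurretRange.
; Sphere overlaps add any actor as a potential target and signal the BP_ProjectileTurretAIController, while exits remove only BP_Enemy actors.
; LookAtLocation is an empty function, and the turret itself contains no aiming or firing logic.
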(event OnComponentBeginOverlap(TurretRangeCollisionSphere)
  (params (OverlappedComponent :type Primitive%20Component%20Object%20Reference) (OtherActor :type Actor%20Object%20Reference) (OtherComp :type Primitive%20Component%20Object%20Reference) (OtherBodyIndex :type Integer) (bFromSweep :type Boolean) (SweepResult :type Hit%20Result%20Structure%20%28by%20ref%29))
  (bind _asbp_projectile_turret_aicontroller (Utilities|Casting|CastToBP_ProjectileTurretAIController (Pawn|GetController)))
  (Default|AddPotentialTarget _asbp_projectile_turret_aicontroller OtherActor)
  (Default|EventTargetsinRange _asbp_projectile_turret_aicontroller))

(event OnComponentEndOverlap(TurretRangeCollisionSphere)
  (params (OverlappedComponent :type Primitive%20Component%20Object%20Reference) (OtherActor :type Actor%20Object%20Reference) (OtherComp :type Primitive%20Component%20Object%20Reference) (OtherBodyIndex :type Integer))
  (bind _asbp_projectile_turret_aicontroller (Utilities|Casting|CastToBP_ProjectileTurretAIController (Pawn|GetController)))
  (bind _asbp_enemy (Utilities|Casting|CastToBP_Enemy OtherActor))
  (Default|RemoveTarget _asbp_projectile_turret_aicontroller _asbp_enemy))

(event EventBeginPlay
  (|CallParentFunction) ; This node is disabled and will not be called.\nDrag off pins to build functionality.
)

(event Collision|EventActorBeginOverlap
  (params (OtherActor :type Actor%20Object%20Reference))
  (|CallParentFunction OtherActor) ; This node is disabled and will not be called.\nDrag off pins to build functionality.
)

(event EventTick
  (params (DeltaSeconds :type Float%20%28single-precision%29))
  (|CallParentFunction DeltaSeconds) ; This node is disabled and will not be called.\nDrag off pins to build functionality.
)

(fn ConstructionScript
  (|CallParentFunction)
  (Components|Sphere|SetSphereRadius (Variables|Turret|GetTurretRangeCollisionSphere) (Variables|Turret|GetTurretRange) true))

(fn LookatLocation
  (params (LookAt :type Vector)))