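; BP_Placeable is a board placeable that either starts in the world, occupying its tiles on BeginPlay, or is positioned with the cursor.
; While placing, Tick snaps it to the component hit under the cursor and calls EditMaterial, an empty stub, over occupied tiles.
; CheckBoardCollision finds TileComponents through overlapping capsules' attach parents and reports occupancy.
; StopPlacing commits only on unoccupied tiles, then marks them occupied.
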(event Custom|Start%20Placing
  (params (Controller :type Player%20Controller%20Object%20Reference))
  (Variables|Default|SetController_0 Controller)
  (Variables|Default|SetIsBeingPlaced true)
  (CallFunction|EditMaterial))

(event Custom|Stop%20Placing
  (bind (_isboardocuupied _overlappingtiles) (CallFunction|CheckBoardCollision))
  (if (not _isboardocuupied)
    (Variables|Default|SetIsBeingPlaced false)
    (for _array_element _overlappingtiles
      (Class|TileComponent|SetIsOccupied _array_element true))))

(event EventBeginPlay
  ;[1 1 1] For placeables dropped in the world
  (if (not (Variables|Default|GetIsBeingPlaced))
    (for _array_element (.OverlappingTiles (CallFunction|CheckBoardCollision))
      (Class|TileComponent|SetIsOccupied _array_element true))))

(event Collision|EventActorBeginOverlap
  (params (OtherActor :type Actor%20Object%20Reference)))

(event EventTick
  (params (DeltaSeconds :type Float%20%28single-precision%29))
  (bind _controller_0 (Variables|Default|GetController_0))
  (bind _object_types (Variables|Default|GetObject%20Types))
  (bind _hitresult (Class|PlayerController|GetHitResultUnderCursorforObjects _controller_0 _object_types true))
  (bind _hitcomponent (Collision|BreakHitResult _hitresult))
  (if (Variables|Default|GetIsBeingPlaced)
    (if (Utilities|IsValid _hitcomponent)
      (Transformation|SetActorLocation (Transformation|GetWorldLocation _hitcomponent) false false)
      (if (.IsBoardOcuupied (CallFunction|CheckBoardCollision))
        (CallFunction|EditMaterial)))))

(fn ConstructionScript)

(fn EditMaterial)

(fn CheckBoardCollision
  (for _array_element (Class|Actor|GetOverlappingComponents self)
    (bind _ascapsule_collision (Utilities|Casting|CastToCapsuleComponent _array_element))
    (bind _astile_component (Utilities|Casting|CastToTileComponent (Transformation|GetAttachParent _ascapsule_collision)))
    (Utilities|Array|Add (LocalVariables|GetTileArray) _astile_component)
    (LocalVariables|SetResult (or (Class|TileComponent|GetIsOccupied _astile_component) (LocalVariables|GetResult))))
  (return (LocalVariables|GetResult) (LocalVariables|GetTileArray)))